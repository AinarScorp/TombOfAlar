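; Ambusher enemy character that detects the player on sphere overlap or when damaged, can play teleport-style jumps, and can slow the player.
; It extends parent enemy logic for damage, death, attack toggling and slowing, adding sound cues and a short debounce on the hit sound.
; It registers with the player's slowing-actor list and unregisters on death; its hits send a zero-damage message.
; Jumps use start and finish sections of one montage.
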(event `self.SphereComponent.OnComponentBeginOverlap`
  (params (OverlappedComponent :type "PrimitiveComponent Object Reference") (OtherActor :type "Actor Object Reference") (OtherComp :type "PrimitiveComponent Object Reference") (OtherBodyIndex :type Integer) (bFromSweep :type Boolean) (SweepResult :type "HitResult Structure (by ref)"))
  (if (== OtherActor (`GameplayStatics.GetPlayerCharacter` 0))
    (`self.OnPlayerDetected` OtherActor)))

(event `self.TakeDamage`
  (params (damage :type "Float (single-precision)") (HitPoint :type "Vector Structure"))
  (`parent.TakeDamage` damage HitPoint)
  (`|ExecutionSequence`
    (:`then_0`
      (`self.OnPlayerDetected` (`GameplayStatics.GetPlayerCharacter` 0)))
    (:`then_1`
      (if (not (`self.ShotDupe`))
        (`GameplayStatics.PlaySoundAtLocation` "/Game/_Game/Blueprints/Sounds/Hit/SFX_Hit.SFX_Hit" (`SceneComponent.K2_GetComponentLocation` (`self.CapsuleComponent`)) (struct) 1.0 1.0 0.0 null null null null)
        (set `self.ShotDupe` true)
        (`KismetSystemLibrary.Delay` 0.2)
        (set `self.ShotDupe` false)))))

(event `self.DamagePlayer`
  (params (Player :type "Actor Object Reference") (HitLocation :type "Vector Structure"))
  (`self.OnHitPlayer`)
  (message `Damageable.TakeDamage` Player 0.0 HitLocation))

(event `self.ToggleJump`
  (params (Disappear :type Boolean))
  (`GameplayStatics.PlaySoundAtLocation` "/Game/_Game/Blueprints/Sounds/Ambusher/SFX_Overheat.SFX_Overheat" (`SceneComponent.K2_GetComponentLocation` (`self.CapsuleComponent`)) (struct) 1.0 1.0 0.0 null null null null)
  (`self.PlayAnimMontage` (`self.JumpMontage`) 1.0 (select `bool` Disappear :`false` "TeleportFinish" :`true` "TeleportStart" :!type "Name")))

(event `self.StartSlowingPlayer`
  (bind _asbp_third_person_character (`/Game/_Game/Library/BP_GameSpecif.GetThirdPersonPlayer`))
  (`parent.StartSlowingPlayer`)
  (`/Game/_Game/Blueprints/Characters/BP_ThirdPersonCharacter.LightSound` _asbp_third_person_character)
  (`/Game/_Game/Blueprints/Characters/BP_ThirdPersonCharacter.ModifySlowingActorList` _asbp_third_person_character self true))

(fn `ExecuteDeath`
  (params (KilledByPlayer :type Boolean))
  (returns (ReturnValue :type Boolean))
  (`parent.ExecuteDeath` KilledByPlayer)
  (`/Game/_Game/Blueprints/Characters/BP_ThirdPersonCharacter.ModifySlowingActorList` (`/Game/_Game/Library/BP_GameSpecif.GetThirdPersonPlayer`) self false)
  (`GameplayStatics.PlaySoundAtLocation` "/Game/_Game/Blueprints/Sounds/RatDeath/SFX_RatDeath.SFX_RatDeath" (`SceneComponent.K2_GetComponentLocation` (`self.CapsuleComponent`)) (struct) 1.0 1.0 0.0 null null null null)
  (return true))

(fn `ToggleAttackExecution`
  (params (TurnOn :type Boolean))
  (returns (ReturnValue :type Boolean))
  (bind _returnvalue (`parent.ToggleAttackExecution` TurnOn))
  (if (`local.TurnOn`)
    (`GameplayStatics.PlaySoundAtLocation` "/Game/_Game/Blueprints/Sounds/Ambusher/SFX_Chain.SFX_Chain" (`SceneComponent.K2_GetComponentLocation` (`self.CapsuleComponent`)) (struct) 1.0 1.0 0.0 null null null null))
  (return _returnvalue))

(fn `UserConstructionScript`)