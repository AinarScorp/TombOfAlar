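; Base Blueprint for horde enemies, apparently rats, adding squeak, hit and death audio and damaging the player.
; From BeginPlay it loops a squeak at random intervals while health remains.
; TakeDamage calls the parent and throttles the hit sound with a short ShotDupe gate, while DamagePlayer forwards damage to the player by message.
; ExecuteDeath calls the parent, then spawns on-death objects and plays a death sound only for player kills.
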(event `self.ReceiveBeginPlay`
  (`GameplayStatics.PlaySoundAtLocation` "/Game/_Game/Blueprints/Sounds/RatSqueek/SFX_Squeek.SFX_Squeek" (`SceneComponent.K2_GetComponentLocation` (`self.CapsuleComponent`)) (struct) 1.0 1.0 0.0 null null null null :!label _label)
  (`KismetSystemLibrary.Delay` (`KismetMathLibrary.RandomFloatInRange` 0.5 3.0))
  (if (not (<= (`self.CurrentHealth`) 0.0))
    (goto _label)))

(event `self.TakeDamage`
  (params (damage :type "Float (single-precision)") (HitPoint :type "Vector Structure"))
  (`parent.TakeDamage` damage HitPoint)
  (if (not (`self.ShotDupe`))
    (`GameplayStatics.PlaySoundAtLocation` "/Game/_Game/Blueprints/Sounds/Hit/SFX_Hit.SFX_Hit" (`SceneComponent.K2_GetComponentLocation` (`self.CapsuleComponent`)) (struct) 1.0 1.0 0.0 null null null null)
    (set `self.ShotDupe` true)
    (`KismetSystemLibrary.Delay` 0.2)
    (set `self.ShotDupe` false)))

(event `self.DamagePlayer`
  (params (Player :type "Actor Object Reference") (HitLocation :type "Vector Structure"))
  (message `Damageable.TakeDamage` Player (`self.Damage`) HitLocation))

(fn `ExecuteDeath`
  (params (KilledByPlayer :type Boolean))
  (returns (ReturnValue :type Boolean))
  (`parent.ExecuteDeath` KilledByPlayer)
  (if KilledByPlayer
    (`self.SpawnOnDeathObjects`)
    (`GameplayStatics.PlaySoundAtLocation` "/Game/_Game/Blueprints/Sounds/RatDeath/SFX_RatDeath.SFX_RatDeath" (`SceneComponent.K2_GetComponentLocation` (`self.CapsuleComponent`)) (struct) 1.0 1.0 0.0 null null null null))
  (return false))

(fn `UserConstructionScript`)