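; Skeleton tank enemy character that adds tank-specific sounds, hit effects, jump montages and a health bar to its parent's damage, attack and death logic.
; It registers in the horde subsystem's tank list on spawn and removes itself on death.
; A looping timer plays its ambient sound until death.
; Each Tick rotates the widget health bar using the camera's direction, with fixed yaw, and pushes current health against a hardcoded maximum.
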(event `self.ReceiveTick`
  (params (DeltaSeconds :type "Float (single-precision)"))
  (bind _hpbar (`self.HpBar`))
  (bind (_returnvalue_roll _returnvalue_pitch) (`KismetMathLibrary.BreakRotator` (`KismetMathLibrary.FindLookAtRotation` (`SceneComponent.K2_GetComponentLocation` _hpbar) (`self.K2_GetActorLocation` (`GameplayStatics.GetPlayerCameraManager` 0)))))
  (`/Engine/EditorBlueprintResources/StandardMacros.IsValid` _hpbar
    (:`Is Valid`
      (`SceneComponent.K2_SetWorldRotation` (`self.HpBar`) (`KismetMathLibrary.MakeRotator` _returnvalue_roll _returnvalue_pitch 90.0) false false)
      (`/Game/_Game/UI/WBP_TankHP.SetHealth` (`self.HealthBarRef`) (`self.CurrentHealth`) 100.0))))

(event `self.ReceiveBeginPlay`
  (`|ExecutionSequence`
    (:`then_0`
      (`KismetArrayLibrary.Array_Add` (`EnemyHordeSubsystem.ListOfTankEnemies` (subsystem `EnemyHordeSubsystem`)) self))
    (:`then_1`
      (bind _returnvalue (`KismetSystemLibrary.K2_SetTimerDelegate` (delegate `LoopTankSound`) 3.0 true 0.1))
      (set `self.SoundLoopSound` _returnvalue))
    (:`then_2`
      (bind _aswbp_tank_hp (cast `/Game/_Game/UI/WBP_TankHP` (`WidgetComponent.GetWidget` (`self.HpBar`))))
      (set `self.HealthBarRef` _aswbp_tank_hp))))

(event `LoopTankSound`
  (`GameplayStatics.PlaySoundAtLocation` "/Game/_Game/Blueprints/Sounds/BoneBreak/SFX_Tank.SFX_Tank" (`SceneComponent.K2_GetComponentLocation` (`self.CapsuleComponent`)) (struct) 1.0 1.0 0.0 null null null null))

(event `self.TakeDamage`
  (params (damage :type "Float (single-precision)") (HitPoint :type "Vector Structure"))
  (`parent.TakeDamage` damage HitPoint)
  (`GameplayStatics.PlaySoundAtLocation` "/Game/_Game/Blueprints/Sounds/Hit/SFX_Hit.SFX_Hit" (`SceneComponent.K2_GetComponentLocation` (`self.CapsuleComponent`)) (struct) 1.0 1.0 0.0 null null null null)
  (`GameplayStatics.SpawnEmitterAtLocation` "/Game/FXVarietyPack/Particles/P_ky_hit1.P_ky_hit1" HitPoint))

(event `/Game/_Game/Interfaces/BI_TankEnemy.PerformJump`
  (`self.PlayAnimMontage` "/Game/_Game/Animations/Montages/SkeletonTank/AM_SkeletonTankJump.AM_SkeletonTankJump" 0.5))

(event `/Game/_Game/Interfaces/BI_TankEnemy.InAir`
  (`self.PlayAnimMontage` "/Game/_Game/Animations/Montages/SkeletonTank/AM_SkeletonTankInAir.AM_SkeletonTankInAir"))

(event `/Game/_Game/Interfaces/BI_TankEnemy.FinishJump`
  (`self.PlayAnimMontage` "/Game/_Game/Animations/Montages/SkeletonTank/AM_SkeletonTankFinishJump.AM_SkeletonTankFinishJump"))

(fn `ExecuteDeath`
  (params (KilledByPlayer :type Boolean))
  (returns (ReturnValue :type Boolean))
  (bind _returnvalue (`parent.ExecuteDeath` KilledByPlayer))
  (`KismetSystemLibrary.K2_ClearAndInvalidateTimerHandle` (`self.SoundLoopSound`))
  (`ActorComponent.K2_DestroyComponent` (`self.HpBar`))
  (if KilledByPlayer
    (`GameplayStatics.PlaySoundAtLocation` "/Game/_Game/Blueprints/Sounds/ShooterDeath/SFX_TankDeath.SFX_TankDeath" (`SceneComponent.K2_GetComponentLocation` (`self.CapsuleComponent`)) (struct) 1.0 1.0 0.0 null null null null))
  (`KismetArrayLibrary.Array_RemoveItem` (`EnemyHordeSubsystem.ListOfTankEnemies` (subsystem `EnemyHordeSubsystem`)) self)
  (return _returnvalue))

(fn `PerformAttack`
  (returns (ReturnValue :type Boolean))
  (bind _returnvalue (`parent.PerformAttack`))
  (`GameplayStatics.PlaySoundAtLocation` "/Game/_Game/Blueprints/Sounds/ShooterAttack/SFX_TankAttack.SFX_TankAttack" (`SceneComponent.K2_GetComponentLocation` (`self.CapsuleComponent`)) (struct) 1.0 1.0 0.0 null null null null)
  (return _returnvalue))

(fn `UserConstructionScript`)