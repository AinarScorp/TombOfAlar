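; Skeleton archer enemy character that carries an animated bow and shoots at the player.
; On begin play it spawns an archer weapon on the bow and registers with the enemy horde subsystem's archer list, leaving it on death.
; Attacking plays the bow animation and sound, while FireWeapon triggers the weapon aimed at player 0.
; Hit effects, a player-kill death sound and randomly timed ambient sounds while alive layer onto parent behavior.
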(event `self.ReceiveBeginPlay`
  (`|ExecutionSequence`
    (:`then_0`
      (bind _returnvalue (`|SpawnActorFromClass` "/Game/_Game/Blueprints/Actors/Weapons/AI_Weapons/AI_Archer_Weapon/BP_ArcherWeapon.BP_ArcherWeapon_C" (`self.GetTransform`) "Undefined" "MultiplyWithRoot" null null))
      (bind _output_get (set `self.Weapon` _returnvalue))
      (`self.K2_AttachToComponent` _output_get (`self.Bow`) "Bow6" "SnapToTarget" "SnapToTarget" "KeepRelative" true)
      (`KismetArrayLibrary.Array_Add` (`EnemyHordeSubsystem.ListOfArchers` (subsystem `EnemyHordeSubsystem`)) self))
    (:`then_1`
      (`GameplayStatics.PlaySoundAtLocation` "/Game/_Game/Blueprints/Sounds/BoneBreak/SFX_Skeleton.SFX_Skeleton" (`SceneComponent.K2_GetComponentLocation` (`self.CapsuleComponent`)) (struct) 1.0 1.0 0.0 null null null null :!label _label)
      (`KismetSystemLibrary.Delay` (`KismetMathLibrary.RandomFloatInRange` 0.5 3.0))
      (if (not (<= (`self.CurrentHealth`) 0.0))
        (goto _label)))))

(event `self.FireWeapon`
  (`Weapon.OnPrimaryPressed` (`self.Weapon`) (`EinarMathLibrary.DirectionToActor` self (`GameplayStatics.GetPlayerCharacter` 0) true) 0.0 self))

(event `self.TakeDamage`
  (params (damage :type "Float (single-precision)") (HitPoint :type "Vector Structure"))
  (`parent.TakeDamage` damage HitPoint)
  (`GameplayStatics.PlaySoundAtLocation` "/Game/_Game/Blueprints/Sounds/Hit/SFX_Hit.SFX_Hit" (`SceneComponent.K2_GetComponentLocation` (`self.CapsuleComponent`)) (struct) 1.0 1.0 0.0 null null null null)
  (`GameplayStatics.SpawnEmitterAtLocation` "/Game/FXVarietyPack/Particles/P_ky_hit1.P_ky_hit1" HitPoint))

(fn `ExecuteDeath`
  (params (KilledByPlayer :type Boolean))
  (returns (ReturnValue :type Boolean))
  (bind _returnvalue (`parent.ExecuteDeath` KilledByPlayer))
  (if KilledByPlayer
    (`GameplayStatics.PlaySoundAtLocation` "/Game/_Game/Blueprints/Sounds/ShooterDeath/SFX_ArcherDeath.SFX_ArcherDeath" (`SceneComponent.K2_GetComponentLocation` (`self.CapsuleComponent`)) (struct) 1.0 1.0 0.0 null null null null))
  (`KismetArrayLibrary.Array_RemoveItem` (`EnemyHordeSubsystem.ListOfArchers` (subsystem `EnemyHordeSubsystem`)) self)
  (return _returnvalue))

(fn `PerformAttack`
  (returns (ReturnValue :type Boolean))
  (`parent.PerformAttack`)
  (`SkeletalMeshComponent.PlayAnimation` (`self.Bow`) "/Game/SkeletonEnemy/Animations/Anim_Bow_Attack.Anim_Bow_Attack" false)
  (`GameplayStatics.PlaySoundAtLocation` "/Game/_Game/Blueprints/Sounds/ShooterAttack/SFX_ShooterAttack.SFX_ShooterAttack" (`SceneComponent.K2_GetComponentLocation` (`self.CapsuleComponent`)) (struct) 1.0 1.0 0.0 null null null null)
  (return true))

(fn `UserConstructionScript`
  (`SceneComponent.K2_AttachToComponent` (`self.Bow`) (`self.Mesh`) "SKT_Bow" "SnapToTarget" "SnapToTarget" "KeepRelative" true))