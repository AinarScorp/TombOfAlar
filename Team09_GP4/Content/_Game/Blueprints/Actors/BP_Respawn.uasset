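; BP_Respawn is a tombstone checkpoint that sets the player's respawn transform on overlap.
; A new activation registers it as current checkpoint, shows a HUD prompt, plays animation and sound, then reveals VFX, which Tick hides when another checkpoint is current.
; RespawnPlayer resets linked actors in ThingsToReset through interface messages and replays tombstone effects.
; The construction script optionally draws debug lines to those linked actors.
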(event `self.ReceiveBeginPlay`
  (set `self.Player` (`/Game/_Game/Library/BP_GameSpecif.GetThirdPersonPlayer`)))

(event `self.Box.OnComponentBeginOverlap`
  (params (OverlappedComponent :type "PrimitiveComponent Object Reference") (OtherActor :type "Actor Object Reference") (OtherComp :type "PrimitiveComponent Object Reference") (OtherBodyIndex :type Integer) (bFromSweep :type Boolean) (SweepResult :type "HitResult Structure (by ref)"))
  (bind _returnvalue_location (`KismetMathLibrary.BreakTransform` (`self.GetTransform`)))
  (bind (_transform_location _transform_rotation) (`KismetMathLibrary.BreakTransform` (`self.Transform`)))
  (bind _player (`self.Player`))
  (if (== OtherActor _player)
    (set `/Game/_Game/Blueprints/Characters/BP_ThirdPersonCharacter.SpawnTransform` (`KismetMathLibrary.MakeTransform` _returnvalue_location _transform_rotation) _player)
    (if (not (== (`/Game/_Game/Blueprints/Characters/BP_ThirdPersonCharacter.CurrentCheckpoint` (`self.Player`)) self))
      (`/Game/_Game/UI/WBP_HUD.CheckpointPrompt` (`/Game/_Game/Blueprints/Characters/BP_ThirdPersonCharacter.HUD` (`self.Player`)))
      (`SkeletalMeshComponent.PlayAnimation` (`self.SkeletalMesh`) "/Game/_Game/Art/Tombstone/AM_TombstoneCollide.AM_TombstoneCollide" false)
      (set `/Game/_Game/Blueprints/Characters/BP_ThirdPersonCharacter.CurrentCheckpoint` self (`self.Player`))
      (`GameplayStatics.PlaySoundAtLocation` "/Game/_Game/Blueprints/Sounds/Tomb/SFX_Checkpoint.SFX_Checkpoint" (`SceneComponent.K2_GetComponentLocation` (`self.SkeletalMesh`)) (struct) 1.0 1.0 0.0 null null null null)
      (`KismetSystemLibrary.Delay` 1.5)
      (`SceneComponent.SetVisibility` (`self.VFX`) true false))))

(event `RespawnPlayer`
  (bind _vfx (`self.VFX`))
  (`self.ResetSpawners`)
  (`SkeletalMeshComponent.PlayAnimation` (`self.SkeletalMesh`) "/Game/_Game/Art/Tombstone/AM_TombstoneRespawn.AM_TombstoneRespawn" false)
  (`SceneComponent.SetVisibility` _vfx false false)
  (`KismetSystemLibrary.Delay` 2.0)
  (`SceneComponent.SetVisibility` _vfx true false))

(event `self.ReceiveTick`
  (params (DeltaSeconds :type "Float (single-precision)"))
  (bind _player (`self.Player`)
    (:`then`
      (bind _currentcheckpoint (`/Game/_Game/Blueprints/Characters/BP_ThirdPersonCharacter.CurrentCheckpoint` _player)
        (:`then`
          (if (!= _currentcheckpoint self)
            (`SceneComponent.SetVisibility` (`self.VFX`) false false)))
        (:`else`)))
    (:`else`)))

(fn `ResetSpawners`
  (for _array_element (`self.ThingsToReset`)
    (message `Resettable.ResetUponPlayerDeath` _array_element)))

(fn `UserConstructionScript`
  (`self.VisualizeConnections`))

(fn `VisualizeConnections`
  (`KismetSystemLibrary.FlushPersistentDebugLines`)
  (if (`self.DrawGizmos`)
    (for _array_element (`self.ThingsToReset`)
      (bind _returnvalue (message `Resettable.GetActor` _array_element))
      (`/Engine/EditorBlueprintResources/StandardMacros.IsValid` _returnvalue
        (:`Is Valid`
          (`KismetSystemLibrary.DrawDebugLine` (`SceneComponent.K2_GetComponentLocation` (`self.GizmoBillboard`)) (`self.K2_GetActorLocation` _returnvalue) (`self.GizmoColor`) 9999999.0 5.0))))))