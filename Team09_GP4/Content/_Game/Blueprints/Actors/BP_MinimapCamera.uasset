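; BP_MinimapCamera is an overhead scene capture actor that follows the player for a minimap view.
; On BeginPlay it caches the BP_ThirdPersonCharacter player and sets the capture component's ortho width from ZoomLevel.
; Each Tick it moves the SceneCaptureComponent2D, with sweep enabled, to a fixed height above the player's location.
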(event `self.ReceiveBeginPlay`
  (bind _asbp_third_person_character (cast `/Game/ThirdPerson/Blueprints/BP_ThirdPersonCharacter` (`GameplayStatics.GetPlayerCharacter` 0)))
  (set `self.PlayerRef` _asbp_third_person_character)
  (set `SceneCaptureComponent2D.OrthoWidth` (`self.ZoomLevel`) (`self.SceneCaptureComponent2D`)))

(event `self.ReceiveTick`
  (params (DeltaSeconds :type "Float (single-precision)"))
  (`SceneComponent.K2_SetWorldLocation` (`self.SceneCaptureComponent2D`) (+ (`self.K2_GetActorLocation` (`self.PlayerRef`)) (0.0 0.0 1000.0)) true false))

(fn `UserConstructionScript`)