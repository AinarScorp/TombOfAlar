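; BP_Explosion is a short-lived explosion actor that deals damage and plays a VFX.
; On BeginPlay it keeps collision off briefly, then enables it and activates the effect, later destroying the collision component and finally itself.
; The overlap handler sends a fixed-damage TakeDamage message with a zero hit point.
; A DoOnce gate limits damage to the first valid overlapping actor.
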(event `self.ReceiveBeginPlay`
  (`PrimitiveComponent.SetCollisionEnabled` (`self.Collision`) "NoCollision")
  (`KismetSystemLibrary.Delay` 0.05)
  (`PrimitiveComponent.SetCollisionEnabled` (`self.Collision`) "QueryAndPhysics")
  (`ActorComponent.Activate` (`self.ExplosionVFX`) false)
  (`KismetSystemLibrary.Delay` 0.75)
  (`ActorComponent.K2_DestroyComponent` (`self.Collision`))
  (`KismetSystemLibrary.Delay` 1.0)
  (`self.K2_DestroyActor`))

(event `self.Collision.OnComponentBeginOverlap`
  (params (OverlappedComponent :type "PrimitiveComponent Object Reference") (OtherActor :type "Actor Object Reference") (OtherComp :type "PrimitiveComponent Object Reference") (OtherBodyIndex :type Integer) (bFromSweep :type Boolean) (SweepResult :type "HitResult Structure (by ref)"))
  (`/Engine/EditorBlueprintResources/StandardMacros.IsValid` OtherActor
    (:`Is Valid`
      (if (not (`self.DoOnce`))
        (set `self.DoOnce` true)
        (message `Damageable.TakeDamage` OtherActor 20.0 (0.0 0.0 0.0))))))

(fn `UserConstructionScript`)