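; Siphon VFX actor that flies from its own location to the third-person player's left wrist socket over a given duration, then destroys itself.
; StartMoving caches the start point and player mesh and starts a looping timer at the frame delta interval, apparently driving MoveTowardsEnd.
; That function lerps toward the live socket position using elapsed time over duration.
; An older timeline-based flight and particle-hiding logic are left disconnected.
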(event `StartMoving`
  (params (SiphonDuration :type "Float (double-precision)"))
  (set `self.Siphon Duration` SiphonDuration)
  (set `self.StartLocation` (`self.K2_GetActorLocation`))
  (set `self.Alpha` 0.0)
  (set `self.PlayerMeshCache` (`Character.Mesh` (`/Game/_Game/Library/BP_GameSpecif.GetThirdPersonPlayer`)))
  (bind _returnvalue (`KismetSystemLibrary.K2_SetTimerDelegate` (`|CreateDelegate` :!event `MoveTowardsEnd`) (`GameplayStatics.GetWorldDeltaSeconds`) true))
  (set `self.MoveTimer` _returnvalue))

(event `self.ReceiveBeginPlay`)

(fn `InreaseAlpha`
  (returns (`0.1` :type "Float (double-precision)"))
  (bind _output_get (set `self.PastTime` (+ (`GameplayStatics.GetWorldDeltaSeconds`) (`self.PastTime`))))
  (bind _output_get_2 (set `self.Alpha` (/ _output_get (`self.Siphon Duration`))))
  (return _output_get_2))

(fn `MoveTowardsEnd`
  (bind _0_1 (`self.InreaseAlpha`))
  (`self.K2_SetActorLocation` (`KismetMathLibrary.VLerp` (`self.StartLocation`) (`SceneComponent.GetSocketLocation` (`self.PlayerMeshCache`) "Wrist_LSocket") _0_1))
  (`self.TryStopMoving`))

(fn `TryStopMoving`
  (if (>= (`self.Alpha`) 1.0)
    (`KismetSystemLibrary.K2_ClearAndInvalidateTimerHandle` (`self.MoveTimer`))
    (`self.K2_DestroyActor`)))

(fn `UserConstructionScript`)