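; BP_DestructableWall is a terrain actor that can be destroyed by damage.
; It copies its starting health into HP on BeginPlay and subtracts incoming damage from it.
; The wall destroys itself when HP reaches zero or below, and otherwise prints the remaining HP as a debug string.
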(event `self.ReceiveBeginPlay`
  (set `self.HP` (`self.StartHP`)))

(event `self.TakeDamage`
  (params (damage :type "Float (single-precision)"))
  (bind _output_get (set `self.HP` (- (`self.HP`) damage)))
  (if (<= _output_get 0.0)
    (`self.K2_DestroyActor`)
    (else
      (`KismetSystemLibrary.PrintString` (`KismetStringLibrary.Conv_DoubleToString` _output_get)))))

(fn `UserConstructionScript`)