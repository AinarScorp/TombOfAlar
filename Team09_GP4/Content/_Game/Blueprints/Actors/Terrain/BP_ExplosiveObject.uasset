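; BP_ExplosiveObject is a destructible terrain actor that explodes when damage depletes its very small health pool.
; On lethal damage it spawns BP_Explosion at the Cube's location, then hides, deactivates and disables collision on its Box and Cube instead of being destroyed.
; ReActivate, called by ResetUponPlayerDeath, restores health, visibility and query-only collision so the object can explode again.
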(event `self.ResetUponPlayerDeath`
  (`self.ReActivate`))

(event `ReActivate`
  (set `self.Exploded` false)
  (set `self.Health` 0.1)
  (`PrimitiveComponent.SetCollisionEnabled` (`self.Box`) "QueryOnly")
  (`PrimitiveComponent.SetCollisionEnabled` (`self.Cube`) "QueryOnly")
  (`ActorComponent.SetActive` (`self.Box`) true false)
  (`ActorComponent.SetActive` (`self.Cube`) true false)
  (`SceneComponent.SetVisibility` (`self.Cube`) true false)
  (`SceneComponent.SetVisibility` (`self.Box`) true false))

(event `self.TakeDamage`
  (params (damage :type "Float (single-precision)") (HitPoint :type "Vector Structure"))
  (bind _box (`self.Box`))
  (bind _cube (`self.Cube`))
  ;[1 1 1] Health
  (if (not (`self.Exploded`))
    (bind _output_get (set `self.Health` (- (`self.Health`) damage)))
    (if (<= _output_get 0.0)
      (`|SpawnActorFromClass` "/Game/_Game/Blueprints/Actors/Terrain/BP_Explosion.BP_Explosion_C" (`KismetMathLibrary.Conv_VectorToTransform` (`SceneComponent.K2_GetComponentLocation` (`self.Cube`))) "AdjustIfPossibleButAlwaysSpawn" "MultiplyWithRoot" null null)
      (set `self.Exploded` true)
      (`SceneComponent.SetVisibility` _box false false)
      (`ActorComponent.SetActive` _box false false)
      (`ActorComponent.SetActive` _cube false false)
      (`SceneComponent.SetVisibility` _cube false false)
      (`PrimitiveComponent.SetCollisionEnabled` (`self.Box`) "NoCollision")
      (`PrimitiveComponent.SetCollisionEnabled` (`self.Cube`) "NoCollision"))))

(fn `GetActor`
  (returns (ReturnValue :type "Actor Object Reference"))
  (return self))

(fn `UserConstructionScript`)