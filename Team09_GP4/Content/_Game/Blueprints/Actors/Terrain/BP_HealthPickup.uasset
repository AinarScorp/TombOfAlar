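; BP_HealthPickup is a health pickup that homes in on the third-person player and heals them on contact.
; Sphere overlap starts a Delay-driven loop that interpolates the actor toward the player while health is at most 99.5, using DeltaSeconds cached from Tick.
; Cube overlap adds HealAmount, without clamping, if health differs from max, then plays sound, vignette and VFX before destroying itself.
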(event `self.ReceiveBeginPlay`
  (bind _returnvalue (`GameplayStatics.GetActorOfClass` "/Game/_Game/Blueprints/Characters/BP_ThirdPersonCharacter.BP_ThirdPersonCharacter_C"))
  (set `self.Player` _returnvalue))

(event `self.ReceiveTick`
  (params (DeltaSeconds :type "Float (single-precision)"))
  (set `self.DeltaSeconds` DeltaSeconds))

(event `self.Cube.OnComponentBeginOverlap`
  (params (OverlappedComponent :type "PrimitiveComponent Object Reference") (OtherActor :type "Actor Object Reference") (OtherComp :type "PrimitiveComponent Object Reference") (OtherBodyIndex :type Integer) (bFromSweep :type Boolean) (SweepResult :type "HitResult Structure (by ref)"))
  (bind _player (`self.Player`))
  (bind _player_2 (`self.Player`))
  (bind _currenthealth (`/Game/_Game/Blueprints/Characters/BP_ThirdPersonCharacter.CurrentHealth` _player))
  (if (== OtherActor (`/Game/_Game/Library/BP_GameSpecif.GetThirdPersonPlayer`))
    (`/Engine/EditorBlueprintResources/StandardMacros.IsValid` _player
      (:`Is Valid`
        (if (not (== (`/Game/_Game/Blueprints/Characters/BP_ThirdPersonCharacter.MaxHealth` _player) _currenthealth))
          (set `/Game/_Game/Blueprints/Characters/BP_ThirdPersonCharacter.CurrentHealth` (+ _currenthealth (`self.HealAmount`)) _player)
          (`GameplayStatics.PlaySoundAtLocation` "/Game/_Game/Blueprints/Sounds/Pickup/SFX_ItemPU.SFX_ItemPU" (`SceneComponent.K2_GetComponentLocation` (`self.Sphere`)) (struct) 1.0 1.0 0.0 null null null null)
          (`/Game/_Game/Blueprints/Characters/BP_ThirdPersonCharacter.HealthPUVignetteLerp` _player_2)
          (`|SpawnActorFromClass` "/Game/_Game/Blueprints/Actors/Terrain/BP_HealthVFX.BP_HealthVFX_C" (`KismetMathLibrary.MakeTransform` (`SceneComponent.K2_GetComponentLocation` (`Character.CapsuleComponent` _player_2))) "Undefined" "MultiplyWithRoot" null null)
          (`self.K2_DestroyActor`))))))

(event `self.Sphere.OnComponentBeginOverlap`
  (params (OverlappedComponent :type "PrimitiveComponent Object Reference") (OtherActor :type "Actor Object Reference") (OtherComp :type "PrimitiveComponent Object Reference") (OtherBodyIndex :type Integer) (bFromSweep :type Boolean) (SweepResult :type "HitResult Structure (by ref)"))
  (bind _player (`self.Player`))
  (bind _returnvalue (`self.K2_GetActorLocation` _player))
  (if (== OtherActor (`/Game/_Game/Library/BP_GameSpecif.GetThirdPersonPlayer`))
    (if (<= (`/Game/_Game/Blueprints/Characters/BP_ThirdPersonCharacter.CurrentHealth` _player) 99.5) :!label _label
      (`/Engine/EditorBlueprintResources/StandardMacros.IsValid` _player
        (:`Is Valid`
          (`self.SmoothMove` _returnvalue)
          (`KismetSystemLibrary.Delay` 0.01)
          (if (not (<= (`KismetMathLibrary.Vector_Distance` _returnvalue (`self.K2_GetActorLocation`)) 0.0))
            (goto _label)))))))

(fn `SmoothMove`
  (params (TargetLocation :type "Vector Structure"))
  (`self.K2_SetActorLocation` (`KismetMathLibrary.VInterpTo` (.location (`self.GetTransform`)) TargetLocation (`self.DeltaSeconds`) (`self.Speed`))))

(fn `UserConstructionScript`)