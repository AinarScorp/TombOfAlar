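; BP_Explosion is a one-shot explosion actor that plays its effects and damages nearby actors as soon as it begins play.
; BeginPlay activates the VFX, plays a sound and triggers a world camera shake at its location.
; A sphere overlap then sends a flat TakeDamage interface message, with a zero hit point, to each actor found.
; The actor destroys itself after a short delay.
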(event `self.ReceiveBeginPlay`
  (bind _returnvalue (`self.K2_GetActorLocation`))
  (`ActorComponent.Activate` (`self.ExplosionVFX`) false)
  (`GameplayStatics.PlaySoundAtLocation` "/Game/_Game/Blueprints/Sounds/Explosion/SFX_Explosion.SFX_Explosion" _returnvalue (struct) 1.0 1.0 0.0 null null null null)
  (`GameplayStatics.PlayWorldCameraShake` "/Game/_Game/Blueprints/Actors/BP_CameraShake1.BP_CameraShake1_C" _returnvalue 0.0 2000.0)
  (bind _outactors (`KismetSystemLibrary.SphereOverlapActors` (`self.K2_GetActorLocation`) 300.0 (`self.Obejcts`)))
  (for _array_element _outactors
    (message `Damageable.TakeDamage` _array_element 20.0 (0.0 0.0 0.0)))
  (`KismetSystemLibrary.Delay` 1.0)
  (`self.K2_DestroyActor`))

(fn `UserConstructionScript`)