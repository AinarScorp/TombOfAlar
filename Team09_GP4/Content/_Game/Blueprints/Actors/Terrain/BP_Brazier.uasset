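; BP_Brazier is a terrain brazier actor that reacts to the player's proximity and registers itself in the player's slowing-actor list.
; Sphere overlap adds or removes it from that list and toggles a chain VFX, with a sound on entry.
; A timeline animates the spotlight's attenuation radius, while a looping per-frame timer drives the chain between brazier and player.
; Damage-and-destroy logic exists but is disconnected.
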(event `self.ReceiveBeginPlay`
  (bind _returnvalue (`GameplayStatics.GetActorOfClass` "/Game/_Game/Blueprints/Characters/BP_ThirdPersonCharacter.BP_ThirdPersonCharacter_C"))
  (set `self.Player` _returnvalue))

(event `self.TakeDamage`
  (params (damage :type "Float (single-precision)") (HitPoint :type "Vector Structure")))

(event `self.Sphere.OnComponentBeginOverlap`
  (params (OverlappedComponent :type "PrimitiveComponent Object Reference") (OtherActor :type "Actor Object Reference") (OtherComp :type "PrimitiveComponent Object Reference") (OtherBodyIndex :type Integer) (bFromSweep :type Boolean) (SweepResult :type "HitResult Structure (by ref)"))
  (bind _player (`self.Player`))
  (if (== OtherActor (`self.Player`))
    (`/Game/_Game/Blueprints/Characters/BP_ThirdPersonCharacter.ModifySlowingActorList` _player self true)
    (`self.ToggleVFX` true)
    (`/Game/_Game/Blueprints/Characters/BP_ThirdPersonCharacter.LightSound` _player)
    (bind (_direction _lightchangevalues) (`Timeline|LightChange` :!label _label)
      (:`Update`
        (`LocalLightComponent.SetAttenuationRadius` (`self.SpotLight`) _lightchangevalues)))))

(event `self.Sphere.OnComponentEndOverlap`
  (params (OverlappedComponent :type "PrimitiveComponent Object Reference") (OtherActor :type "Actor Object Reference") (OtherComp :type "PrimitiveComponent Object Reference") (OtherBodyIndex :type Integer))
  (if (== OtherActor (`self.Player`))
    (`/Game/_Game/Blueprints/Characters/BP_ThirdPersonCharacter.ModifySlowingActorList` (`self.Player`) self false)
    (`self.ToggleVFX` false)
    (goto _label :!via `Reverse`)))

(fn `ToggleVFX`
  (params (TurnOn :type Boolean))
  (bind _chain (`self.Chain`))
  (if TurnOn
    (bind _returnvalue (`KismetSystemLibrary.K2_SetTimerDelegate` (`|CreateDelegate` :!event `VFXTick`) (`GameplayStatics.GetWorldDeltaSeconds`) true))
    (set `self.ChainVFXTimer` _returnvalue)
    (`ActorComponent.Activate` _chain true)
    (else
      (`KismetSystemLibrary.K2_ClearAndInvalidateTimerHandle` (`self.ChainVFXTimer`))
      (`ActorComponent.Deactivate` _chain))))

(fn `UserConstructionScript`)

(fn `VFXTick`
  (bind _chain (`self.Chain`))
  (`FXSystemComponent.SetVectorParameter` _chain "EndLocation" (`self.K2_GetActorLocation` (`GameplayStatics.GetPlayerCharacter` 0)))
  (`FXSystemComponent.SetVectorParameter` _chain "StartLocation" (`self.K2_GetActorLocation`)))