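; BP_LightDebuff is a trigger actor that flags the player as standing in light while inside its Sphere volume.
; On BeginPlay it caches the BP_ThirdPersonCharacter found with GetActorOfClass.
; The Sphere's begin and end overlap events set that character's InLight flag true and false, ignoring all other actors.
; The file itself applies no debuff effect beyond setting this flag.
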(event `self.ReceiveBeginPlay`
  (bind _returnvalue (`GameplayStatics.GetActorOfClass` "/Game/ThirdPerson/Blueprints/BP_ThirdPersonCharacter.BP_ThirdPersonCharacter_C"))
  (set `self.Player` _returnvalue))

(event `self.ReceiveTick`
  (params (DeltaSeconds :type "Float (single-precision)")))

(event `self.Sphere.OnComponentBeginOverlap`
  (params (OverlappedComponent :type "PrimitiveComponent Object Reference") (OtherActor :type "Actor Object Reference") (OtherComp :type "PrimitiveComponent Object Reference") (OtherBodyIndex :type Integer) (bFromSweep :type Boolean) (SweepResult :type "HitResult Structure (by ref)"))
  (bind _player (`self.Player`))
  (if (== OtherActor _player)
    (`/Engine/EditorBlueprintResources/StandardMacros.IsValid` _player
      (:`Is Valid`
        (set `/Game/ThirdPerson/Blueprints/BP_ThirdPersonCharacter.InLight` true _player)))))

(event `self.Sphere.OnComponentEndOverlap`
  (params (OverlappedComponent :type "PrimitiveComponent Object Reference") (OtherActor :type "Actor Object Reference") (OtherComp :type "PrimitiveComponent Object Reference") (OtherBodyIndex :type Integer))
  (bind _player (`self.Player`))
  (if (== OtherActor _player)
    (`/Engine/EditorBlueprintResources/StandardMacros.IsValid` _player
      (:`Is Valid`
        (set `/Game/ThirdPerson/Blueprints/BP_ThirdPersonCharacter.InLight` false _player)))))

(fn `UserConstructionScript`)