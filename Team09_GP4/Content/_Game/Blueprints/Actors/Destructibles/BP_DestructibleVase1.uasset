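; BP_DestructibleVase1 is a destructible vase prop that breaks apart when damage brings its Health to zero or below.
; On breaking it activates the Rubble component and removes the intact mesh and Box component.
; It then enables physics on the broken mesh and pushes it away from player 0 with a mass-independent force.
; The actor destroys itself after a short delay.
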(event `self.TakeDamage`
  (params (damage :type "Float (single-precision)") (HitPoint :type "Vector Structure") (damageType :type "GameDamageType Enum" :default "PLAYER"))
  (bind _sm_prop_vase_broken_01 (`self.SM_Prop_Vase_Broken_01`))
  ;[1 1 1] Health
  (bind _output_get (set `self.Health` (- (`self.Health`) damage)))
  (if (<= _output_get 0.0)
    (`ActorComponent.Activate` (`self.Rubble`) false)
    (`ActorComponent.K2_DestroyComponent` (`self.SM_Prop_Vase_05`))
    (`ActorComponent.K2_DestroyComponent` (`self.Box`))
    (`PrimitiveComponent.SetSimulatePhysics` _sm_prop_vase_broken_01 true)
    (`PrimitiveComponent.AddForce` _sm_prop_vase_broken_01 (* (`KismetMathLibrary.GetDirectionUnitVector` (`self.K2_GetActorLocation` (`GameplayStatics.GetPlayerCharacter` 0)) (`self.K2_GetActorLocation`)) 50000) "None" true)
    (`KismetSystemLibrary.Delay` 1.0)
    (`self.K2_DestroyActor`)))

(fn `UserConstructionScript`)