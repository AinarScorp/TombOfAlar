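; BP_DestructibleCrystal is a breakable crystal prop that can drop a reward actor when destroyed.
; Its TakeDamage event subtracts from Health and, at zero or below, plays a break sound at the hit point and activates the Rubble component.
; If ShouldDropReward is set, it spawns ActorToDrop in its place.
; It removes the mesh and box immediately, then destroys itself after a short delay.
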(event `self.TakeDamage`
  (params (damage :type "Float (single-precision)") (HitPoint :type "Vector Structure"))
  ;[1 1 1] Health
  (bind _output_get (set `self.Health` (- (`self.Health`) damage)))
  (if (<= _output_get 0.0)
    (`GameplayStatics.PlaySoundAtLocation` "/Game/_Game/Blueprints/Sounds/BreakVase/SFX_BreakVase.SFX_BreakVase" HitPoint (struct) 1.0 1.0 0.0 null null null null)
    (`ActorComponent.Activate` (`self.Rubble`) false)
    (if (`self.ShouldDropReward`)
      (`|SpawnActorFromClass` (`self.ActorToDrop`) (`KismetMathLibrary.MakeTransform` (`self.K2_GetActorLocation`) (`self.K2_GetActorRotation`)) "Undefined" "MultiplyWithRoot" null null))
    (`ActorComponent.K2_DestroyComponent` (`self.SM_Prop_Crystals_03`))
    (`ActorComponent.K2_DestroyComponent` (`self.Box`))
    (`KismetSystemLibrary.Delay` 1.0)
    (`self.K2_DestroyActor`)))

(fn `UserConstructionScript`)