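; BP_Collectible is a pickup actor that the player collects by walking into it.
; On BeginPlay it takes a random yaw and a random mesh from MeshArr, though the random index never reaches the last entry when there are several.
; When the player character overlaps its Box, it notifies the HUD through BP_ThirdPersonCharacter, plays a crystal pickup sound and destroys itself.
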(event `self.ReceiveBeginPlay`
  (bind _mesharr (`self.MeshArr`))
  (`self.K2_SetActorRotation` (`KismetMathLibrary.MakeRotator` 0.0 0.0 (* (`KismetMathLibrary.RandomFloat`) 360.0)))
  (`StaticMeshComponent.SetStaticMesh` (`self.SM_Item_Chr_Shrooms_01`) (`|GetArrayItem` _mesharr (`KismetMathLibrary.RandomInteger` (- (`KismetArrayLibrary.Array_Length` _mesharr) 1)))))

(event `self.Box.OnComponentBeginOverlap`
  (params (OverlappedComponent :type "PrimitiveComponent Object Reference") (OtherActor :type "Actor Object Reference") (OtherComp :type "PrimitiveComponent Object Reference") (OtherBodyIndex :type Integer) (bFromSweep :type Boolean) (SweepResult :type "HitResult Structure (by ref)"))
  (bind _returnvalue (`GameplayStatics.GetPlayerCharacter` 0))
  (if (== OtherActor _returnvalue)
    (bind _asbp_third_person_character (cast `/Game/_Game/Blueprints/Characters/BP_ThirdPersonCharacter` _returnvalue))
    (`/Game/_Game/UI/WBP_HUD.PickedUpCollectable` (`/Game/_Game/Blueprints/Characters/BP_ThirdPersonCharacter.HUD` _asbp_third_person_character))
    (`GameplayStatics.PlaySoundAtLocation` "/Game/_Game/Blueprints/Sounds/Pickup/SFX_CrystalPU.SFX_CrystalPU" (`SceneComponent.K2_GetComponentLocation` (`self.Box`)) (struct) 1.0 1.0 0.0 null null null null)
    (`self.K2_DestroyActor`)))

(fn `UserConstructionScript`)