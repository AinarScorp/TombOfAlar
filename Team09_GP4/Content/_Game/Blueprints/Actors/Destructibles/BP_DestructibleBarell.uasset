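; Destructible barrel actor that loses health on TakeDamage and breaks at zero.
; Breaking activates the Rubble component, removes Cube and Box, optionally drops a reward actor and triggers a child-actor enemy spawner for a rat.
; The break sound is gated by a PotBreaking flag on the player character, so barrels seeing it set stay silent.
; The actor destroys itself after a short delay.
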(event `self.TakeDamage`
  (params (damage :type "Float (single-precision)") (HitPoint :type "Vector Structure"))
  (bind _player (`self.Player`))
  ;[1 1 1] Health
  (bind _output_get (set `self.Health` (- (`self.Health`) damage)))
  (if (<= _output_get 0.0)
    (if (not (`/Game/_Game/Blueprints/Characters/BP_ThirdPersonCharacter.PotBreaking` _player))
      (set `/Game/_Game/Blueprints/Characters/BP_ThirdPersonCharacter.PotBreaking` true _player)
      (`/Game/_Game/Blueprints/Characters/BP_ThirdPersonCharacter.PotSoundReset` _player)
      (`GameplayStatics.PlaySoundAtLocation` "/Game/_Game/Blueprints/Sounds/SFX_Break.SFX_Break" HitPoint (struct) 1.0 1.0 0.0 null null null null))
    (`ActorComponent.Activate` (`self.Rubble`) false)
    (`ActorComponent.K2_DestroyComponent` (`self.Cube`))
    (`ActorComponent.K2_DestroyComponent` (`self.Box`))
    (if (`self.ShouldDropReward`)
      (`|SpawnActorFromClass` (`self.ActorToDrop`) (`KismetMathLibrary.MakeTransform` (`self.K2_GetActorLocation`) (`self.K2_GetActorRotation`)) "Undefined" "MultiplyWithRoot" null null))
    (if (`self.ShouldSpawnRat`)
      (`KismetSystemLibrary.Delay` 0.1)
      (bind _asbp_enemy_spawner (cast `/Game/_Game/Blueprints/Actors/Spawner/BP_EnemySpawner` (`ChildActorComponent.ChildActor` (`self.Spawner`))))
      (`EnemySpawner.TriggerSpawner` _asbp_enemy_spawner))
    (`KismetSystemLibrary.Delay` 1.0)
    (`self.K2_DestroyActor`)))

(event `self.ReceiveBeginPlay`
  (bind _returnvalue (`GameplayStatics.GetActorOfClass` "/Game/_Game/Blueprints/Characters/BP_ThirdPersonCharacter.BP_ThirdPersonCharacter_C"))
  (set `self.Player` _returnvalue))

(fn `UserConstructionScript`)