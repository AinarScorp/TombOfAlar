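; BP_DestructibleVase is a breakable vase prop that can drop a reward or trigger an enemy spawn when destroyed.
; TakeDamage depletes Health, then plays break sound and rubble, removes the intact mesh and box, and launches the physics-simulated broken mesh away from the player.
; It sets a VaseBreaking flag on the player and calls its sound reset.
; Optional flags spawn ActorToDrop or trigger the child-actor spawner before the delayed self-destroy.
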(event `self.TakeDamage`
  (params (damage :type "Float (single-precision)") (HitPoint :type "Vector Structure"))
  (bind _sm_prop_vase_broken_01 (`self.SM_Prop_Vase_Broken_01`))
  (bind _player (`self.Player`))
  ;[1 1 1] Health
  (bind _output_get (set `self.Health` (- (`self.Health`) damage)))
  (if (<= _output_get 0.0)
    (if (not (`/Game/_Game/Blueprints/Characters/BP_ThirdPersonCharacter.VaseBreaking` _player))
      (set `/Game/_Game/Blueprints/Characters/BP_ThirdPersonCharacter.VaseBreaking` true _player)
      (`/Game/_Game/Blueprints/Characters/BP_ThirdPersonCharacter.VaseSoundReset` _player))
    (`GameplayStatics.PlaySoundAtLocation` "/Game/_Game/Blueprints/Sounds/BreakVase/SFX_BreakVase.SFX_BreakVase" HitPoint (struct) 1.0 1.0 0.0 null null null null)
    (`ActorComponent.Activate` (`self.Rubble`) false)
    (`ActorComponent.K2_DestroyComponent` (`self.SM_Prop_Vase_05`))
    (`ActorComponent.K2_DestroyComponent` (`self.Box`))
    (`PrimitiveComponent.SetSimulatePhysics` _sm_prop_vase_broken_01 true)
    (`PrimitiveComponent.AddForce` _sm_prop_vase_broken_01 (* (`KismetMathLibrary.GetDirectionUnitVector` (`self.K2_GetActorLocation` (`GameplayStatics.GetPlayerCharacter` 0)) (`self.K2_GetActorLocation`)) 80000) "None" true)
    (if (`self.ShouldDropReward`)
      (`|SpawnActorFromClass` (`self.ActorToDrop`) (`KismetMathLibrary.MakeTransform` (`self.K2_GetActorLocation`) (`self.K2_GetActorRotation`)) "Undefined" "MultiplyWithRoot" null null))
    (if (`self.ShouldSpawnARat`)
      (`KismetSystemLibrary.Delay` 0.1)
      (bind _asbp_enemy_spawner (cast `/Game/_Game/Blueprints/Actors/Spawner/BP_EnemySpawner` (`ChildActorComponent.ChildActor` (`self.Spawner`))))
      (`EnemySpawner.TriggerSpawner` _asbp_enemy_spawner))
    (`KismetSystemLibrary.Delay` 1.0)
    (`self.K2_DestroyActor`)))

(event `self.ReceiveBeginPlay`
  (bind _returnvalue (`GameplayStatics.GetActorOfClass` "/Game/_Game/Blueprints/Characters/BP_ThirdPersonCharacter.BP_ThirdPersonCharacter_C"))
  (set `self.Player` _returnvalue))

(fn `UserConstructionScript`)