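; Weapon pickup actor that unlocks the player character's second weapon when BP_ThirdPersonCharacter overlaps its box.
; If the child actor is a BP_NewWeaponVFX, it passes that effect and its location to the character's unlock visualization.
; It then unlocks the weapon, plays a sound at the child actor and disables box collision.
; An unconnected chain holds input message, player rotation and siphon montage logic that never runs.
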(event `self.Box.OnComponentBeginOverlap`
  (params (OverlappedComponent :type "PrimitiveComponent Object Reference") (OtherActor :type "Actor Object Reference") (OtherComp :type "PrimitiveComponent Object Reference") (OtherBodyIndex :type Integer) (bFromSweep :type Boolean) (SweepResult :type "HitResult Structure (by ref)"))
  (bind _returnvalue (`SceneComponent.K2_GetComponentLocation` (`self.ChildActor`)))
  (bind _asbp_third_person_character (cast `/Game/_Game/Blueprints/Characters/BP_ThirdPersonCharacter` OtherActor))
  (bind _asbp_new_weapon_vfx (cast `/Game/_Game/Blueprints/Actors/Terrain/BP_NewWeaponVFX` (`ChildActorComponent.ChildActor` (`self.ChildActor`)))
    (:`then`
      (`/Game/_Game/Blueprints/Characters/BP_ThirdPersonCharacter.Visualize Unlocking Second Gun` _asbp_third_person_character _returnvalue _asbp_new_weapon_vfx))
    (:`CastFailed`
      _))
  (`/Game/_Game/Blueprints/Characters/BP_ThirdPersonCharacter.UnlockSecondWeapon` _asbp_third_person_character)
  (`GameplayStatics.PlaySoundAtLocation` "/Game/_Game/Blueprints/Sounds/NewWeapon/SFX_NewWeapon.SFX_NewWeapon" _returnvalue (struct) 1.0 1.0 0.0 null null null null)
  (`PrimitiveComponent.SetCollisionEnabled` (`self.Box`) "NoCollision"))

(fn `RotatePlayer`
  (params (Player :type "Actor Object Reference"))
  (bind (_returnvalue_roll _returnvalue_pitch) (`KismetMathLibrary.BreakRotator` (`self.K2_GetActorRotation` Player)))
  (bind (_returnvalue_roll_2 _returnvalue_pitch_2 _returnvalue_yaw) (`KismetMathLibrary.BreakRotator` (`KismetMathLibrary.FindLookAtRotation` (`self.K2_GetActorLocation` Player) (`SceneComponent.K2_GetComponentLocation` (`self.ChildActor`)))))
  (`self.K2_SetActorRotation` Player (`KismetMathLibrary.MakeRotator` _returnvalue_roll _returnvalue_pitch _returnvalue_yaw) false))

(fn `UserConstructionScript`)