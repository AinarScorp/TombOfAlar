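; BP_DefaultWeapon is a weapon actor that adds sound feedback for attacking and overheating.
; The shoot event plays an attack sound at the mesh location, while the primary and secondary fire events are empty.
; Tick watches the first primary spawn data entry and plays an overheat sound once per overheat, re-arming when it clears.
; GetOverheatAmount returns that entry's overheat charge scaled down by a fixed divisor.
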(event `self.OnPrimaryFire`)

(event `self.OnSecondaryFire`)

(event `self.OnShoot`
  (`GameplayStatics.PlaySoundAtLocation` "/Game/_Game/Blueprints/Sounds/SFX_Attack.SFX_Attack" (`SceneComponent.K2_GetComponentLocation` (`self.Mesh`)) (struct) 1.0 1.0 0.0 null null null null))

(event `self.ReceiveTick`
  (params (DeltaSeconds :type "Float (single-precision)"))
  (if (`ProjectileSpawnData.bIsOverheated` (`|GetArrayItem` (`self.PrimarySpawnData`)))
    (if (not (`self.Once`))
      (set `self.Once` true)
      (`GameplayStatics.PlaySoundAtLocation` "/Game/_Game/Blueprints/Sounds/Overheat/SFX_Overheat.SFX_Overheat" (`SceneComponent.K2_GetComponentLocation` (`self.Mesh`)) (struct) 1.0 1.0 0.0 null null null null))
    (else
      (set `self.Once` false))))

(fn `GetOverheatAmount`
  (returns (float :type "Float (double-precision)"))
  (return (/ (`ProjectileSpawnData.OverheatCharge` (`|GetArrayItem` (`self.PrimarySpawnData`))) 10.0)))

(fn `UserConstructionScript`)