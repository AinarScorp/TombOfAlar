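; BP_RifleBullet is a rifle projectile actor with a Niagara trail attached to its sphere on BeginPlay.
; Each tick it turns to face along its ProjectileMovement velocity.
; When new data is applied, it adjusts DestroyTimer linearly by the distance to TargetPoint relative to a fixed baseline, so farther targets give a larger timer value.
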(event `self.OnNewDataApplied`
  (set `self.DestroyTimer` (+ (`self.DestroyTimer`) (* (- (`KismetMathLibrary.Vector_Distance` (`self.TargetPoint`) (`self.K2_GetActorLocation`)) 500.0) 0.0003))))

(event `self.ReceiveBeginPlay`
  (`NiagaraFunctionLibrary.SpawnSystemAttached` "/Game/_Game/VFX/NiagaraSystems/NS_Trail.NS_Trail" (`self.Sphere`) "None" (0.0 0.0 0.0) (struct) "KeepRelativeOffset"))

(event `self.ReceiveTick`
  (params (DeltaSeconds :type "Float (single-precision)"))
  (`self.K2_SetActorRotation` (`KismetMathLibrary.Conv_VectorToRotator` (`KismetMathLibrary.Normal` (`MovementComponent.Velocity` (`self.ProjectileMovement`))))))

(fn `UserConstructionScript`)