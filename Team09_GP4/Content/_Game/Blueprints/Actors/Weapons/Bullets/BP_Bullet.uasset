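; Bullet projectile actor that reports overlaps on its Sphere as hits and plays an impact particle effect.
; On BeginPlay it spawns and attaches a separate BP_BulletVFX actor, then waits one tick before enabling overlap on a custom trace channel, a self-described hacky collision bug fix.
; Sphere overlaps pass the other actor and bullet location to OnHitActor, while OnHitDamagable spawns a scaled-down hit emitter.
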(event `self.ReceiveBeginPlay`
  (bind _returnvalue (`|SpawnActorFromClass` "/Game/_Game/Blueprints/Actors/Terrain/BP_BulletVFX.BP_BulletVFX_C" (`KismetMathLibrary.Conv_VectorToTransform` (`SceneComponent.K2_GetComponentLocation` (`self.Sphere`))) "Undefined" "MultiplyWithRoot" null null))
  (`self.K2_AttachToActor` _returnvalue self "None" "SnapToTarget" "SnapToTarget" "SnapToTarget" true)
  ;[1 1 1] Hacky collision bug fix. Fix by moving the damage to bullet or not allowing collsion if we have no BulletData set
  (`KismetSystemLibrary.DelayUntilNextTick`)
  (`PrimitiveComponent.SetCollisionResponseToChannel` (`self.Sphere`) "ECC_GameTraceChannel5" "ECR_Overlap"))

(event `self.Sphere.OnComponentBeginOverlap`
  (params (OverlappedComponent :type "PrimitiveComponent Object Reference") (OtherActor :type "Actor Object Reference") (OtherComp :type "PrimitiveComponent Object Reference") (OtherBodyIndex :type Integer) (bFromSweep :type Boolean) (SweepResult :type "HitResult Structure (by ref)"))
  (`self.OnHitActor` OtherActor (`self.K2_GetActorLocation`)))

(event `self.OnHitDamagable`
  (params (damagableActor :type "Actor Object Reference") (HitWorldLocation :type "Vector Structure"))
  (`GameplayStatics.SpawnEmitterAtLocation` "/Game/FXVarietyPack/Particles/P_ky_hit1.P_ky_hit1" HitWorldLocation (struct) (0.3 0.3 0.3)))

(fn `UserConstructionScript`)