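; BP_RifleExplosion is an explosive bullet actor that applies hit logic to everything in a radius when destroyed.
; Its Sphere overlap with a BP_RifleBullet works around hit collision, destroying itself a tick later, then the rifle bullet if still valid.
; On destruction, Explode runs a sphere overlap, calling OnHitActor and spawning a small fire impact emitter at its own location for each actor found.
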(event `self.ReceiveTick`
  (params (DeltaSeconds :type "Float (single-precision)"))
  ;[1 0.6563 0.191] Debug
)

(event `self.Sphere.OnComponentBeginOverlap`
  (params (OverlappedComponent :type "PrimitiveComponent Object Reference") (OtherActor :type "Actor Object Reference") (OtherComp :type "PrimitiveComponent Object Reference") (OtherBodyIndex :type Integer) (bFromSweep :type Boolean) (SweepResult :type "HitResult Structure (by ref)"))
  ;[1 0.6672 0.3229] OnHit collision hack
  (bind _asbp_rifle_bullet (cast `/Game/_Game/Blueprints/Actors/Weapons/Bullets/BP_RifleBullet` OtherActor))
  (`KismetSystemLibrary.DelayUntilNextTick`)
  (`self.DestroyBullet`)
  (`/Engine/EditorBlueprintResources/StandardMacros.IsValid` _asbp_rifle_bullet
    (:`Is Valid`
      (`self.DestroyBullet` _asbp_rifle_bullet))))

(event `self.OnDestroyBullet`
  (`self.Explode`))

(fn `Explode`
  (bind _returnvalue (`self.K2_GetActorLocation`))
  (bind _outactors (`KismetSystemLibrary.SphereOverlapActors` (`self.K2_GetActorLocation`) (`self.ExplosionRaduis`) (`|MakeArray` "ObjectTypeQuery9" "ObjectTypeQuery1" "ObjectTypeQuery2" :!type "EObjectTypeQuery Enum") "/Script/Engine.Actor"))
  (for _array_element _outactors
    (`self.OnHitActor` _array_element _returnvalue)
    (`GameplayStatics.SpawnEmitterAtLocation` "/Game/InfinityBladeEffects/Effects/FX_Skill_Leap/P_Skill_Leap_Fire_Impact_Suction.P_Skill_Leap_Fire_Impact_Suction" (+ _returnvalue (0.0 0.0 10.0)) (`self.K2_GetActorRotation`) (0.2 0.2 0.2))))

(fn `UserConstructionScript`)