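; BP_EnemyActivator is a placeable actor that references a set of enemy spawners and shows those links in the level.
; Its construction script flushes persistent debug lines, then, if DrawGizmos is on, draws a long-lasting colored line from its billboard to each valid entry in EnemySpawners.
; The Blueprint contains no runtime logic; BeginPlay is empty and the overlap and tick events are disabled.
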(event `self.ReceiveBeginPlay`)

(fn `UserConstructionScript`
  (`self.VisualizeConnections`))

(fn `VisualizeConnections`
  (`KismetSystemLibrary.FlushPersistentDebugLines`)
  (if (`self.DrawGizmos`)
    (for _array_element (`self.EnemySpawners`)
      (`/Engine/EditorBlueprintResources/StandardMacros.IsValid` _array_element
        (:`Is Valid`
          (`KismetSystemLibrary.DrawDebugLine` (`SceneComponent.K2_GetComponentLocation` (`self.Billboard`)) (`self.K2_GetActorLocation` _array_element) (`self.GizmoColor`) 9999999.0 5.0))))))