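; BP_Walltrigger_Arena is a level trigger that sets off an exploding wall when the player reaches it.
; Its Box overlap checks for player character 0, then calls Explosion on the referenced ExplosionWall if that is valid.
; A disconnected loop that would trigger the SpawnerToTrigger spawners and destroy the actor never runs, so the trigger stays in place and can fire on every overlap.
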(event `self.Box.OnComponentBeginOverlap`
  (params (OverlappedComponent :type "PrimitiveComponent Object Reference") (OtherActor :type "Actor Object Reference") (OtherComp :type "PrimitiveComponent Object Reference") (OtherBodyIndex :type Integer) (bFromSweep :type Boolean) (SweepResult :type "HitResult Structure (by ref)"))
  (bind _explosion_wall (`self.Explosion wall`))
  (if (== OtherActor (`GameplayStatics.GetPlayerCharacter` 0))
    (`/Engine/EditorBlueprintResources/StandardMacros.IsValid` _explosion_wall
      (:`Is Valid`
        (`/Game/_Game/Blueprints/Level/BP_ScriptedEventBridge.Explosion` _explosion_wall)))))

(fn `UserConstructionScript`)