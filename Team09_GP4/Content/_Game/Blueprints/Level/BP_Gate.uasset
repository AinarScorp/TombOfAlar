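; BP_Gate is a level gate that opens once all enemies are killed.
; OnAllEnemiesKilled calls OpenGate, which plays a gate sound at the Box and runs a timeline that drives the Gate actor's relative Z, feeding its world X and Y back in.
; The Box overlap event is empty, and an older player check against the EnemyHordeSubsystem enemy list remains disconnected, as does a lifespan call.
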(event `self.Box.OnComponentBeginOverlap`
  (params (OverlappedComponent :type "PrimitiveComponent Object Reference") (OtherActor :type "Actor Object Reference") (OtherComp :type "PrimitiveComponent Object Reference") (OtherBodyIndex :type Integer) (bFromSweep :type Boolean) (SweepResult :type "HitResult Structure (by ref)")))

(event `Open gate`
  (bind _gate (`self.Gate`))
  (bind (_returnvalue_x _returnvalue_y) (`KismetMathLibrary.BreakVector` (`self.K2_GetActorLocation` _gate)))
  (`GameplayStatics.PlaySoundAtLocation` "/Game/_Game/Blueprints/Sounds/SFX_Gate.SFX_Gate" (`SceneComponent.K2_GetComponentLocation` (`self.Box`)) (struct) 1.0 1.0 0.0 null null null null)
  (bind (_direction _location) (`Timeline|Timeline`)
    (:`Update`
      (`self.K2_SetActorRelativeLocation` _gate (`KismetMathLibrary.MakeVector` _returnvalue_x _returnvalue_y _location) false false))))

(event `self.OnAllEnemiesKilled`
  (`self.Open gate`))

(fn `UserConstructionScript`)