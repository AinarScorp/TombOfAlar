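; BP_Ending is a level trigger that runs the game's ending sequence when the player character overlaps its box.
; The overlap plays a sound, spawns BP_EndingVFX at the player and calls TriggerEndGameMessage.
; After a delay, a timeline drives the end vignette through a material parameter collection.
; The timeline's Update path also creates and animates WBP_EndMenu after another delay, rather than waiting for Finished.
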(event `self.ReceiveBeginPlay`
  (bind _returnvalue (`GameplayStatics.GetActorOfClass` "/Game/_Game/Blueprints/Characters/BP_ThirdPersonCharacter.BP_ThirdPersonCharacter_C"))
  (set `self.Player` _returnvalue))

(event `self.Box.OnComponentBeginOverlap`
  (params (OverlappedComponent :type "PrimitiveComponent Object Reference") (OtherActor :type "Actor Object Reference") (OtherComp :type "PrimitiveComponent Object Reference") (OtherBodyIndex :type Integer) (bFromSweep :type Boolean) (SweepResult :type "HitResult Structure (by ref)"))
  (bind _player (`self.Player`))
  (if (== OtherActor (`self.Player`))
    (`GameplayStatics.PlaySoundAtLocation` "/Game/_Game/Blueprints/Sounds/NewWeapon/SFX_Ending.SFX_Ending" (`SceneComponent.K2_GetComponentLocation` (`self.Box`)) (struct) 1.0 1.0 0.0 null null null null)
    (`|SpawnActorFromClass` "/Game/_Game/Blueprints/Actors/Terrain/BP_EndingVFX.BP_EndingVFX_C" (`KismetMathLibrary.MakeTransform` (`SceneComponent.K2_GetComponentLocation` (`Character.CapsuleComponent` _player))) "Undefined" "MultiplyWithRoot" null null)
    (message `/Game/_Game/Interfaces/BI_Player.TriggerEndGame` _player)
    (`KismetSystemLibrary.Delay` 1.0)
    (bind (_direction _endvignette) (`Timeline|Timeline`)
      (:`Update`
        (`KismetMaterialLibrary.SetScalarParameterValue` "/Game/_Game/Art/Materials/Vignette/Ending/MPC_Vignette_End.MPC_Vignette_End" "VignetteMaskFactor" _endvignette)
        (`KismetSystemLibrary.Delay` 0.5)
        (bind _returnvalue (`|GenericCreateObject` "/Game/_Game/UI/EndMenu/WBP_EndMenu.WBP_EndMenu_C"))
        (`UserWidget.AddToViewport` _returnvalue 0)
        (`UserWidget.PlayAnimation` _returnvalue (`/Game/_Game/UI/EndMenu/WBP_EndMenu.EndAnimation` _returnvalue) 0.0 1 "Forward" 1.0 false)))))

(fn `UserConstructionScript`)