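; BP_ScriptedEventBridge is a level bridge that is blown apart in a scripted explosion.
; Its Explosion event turns on physics for the bridge mesh, plays an explosion sound and applies an impulse built from the Pushpoint's world location plus a large Y offset.
; A breaking sound follows after a short delay, and the actor destroys itself shortly afterward.
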(event `Explosion`
  (`PrimitiveComponent.SetSimulatePhysics` (`self.Bridge`) true)
  (`GameplayStatics.PlaySoundAtLocation` "/Game/_Game/Blueprints/Sounds/Explosion/SFX_Explosion1.SFX_Explosion1" (`SceneComponent.K2_GetComponentLocation` (`self.Bridge`)) (struct) 1.0 1.0 0.0 null null null null)
  (`PrimitiveComponent.AddImpulse` (`self.Bridge`) (+ (`SceneComponent.K2_GetComponentLocation` (`self.Pushpoint`)) (0.0 50000.0 0.0)) "None" false)
  (`KismetSystemLibrary.Delay` 0.2)
  (`GameplayStatics.PlaySoundAtLocation` "/Game/_Game/Blueprints/Sounds/SFX_BreakGate.SFX_BreakGate" (`SceneComponent.K2_GetComponentLocation` (`self.Bridge`)) (struct) 1.0 1.0 0.0 null null null null)
  (`KismetSystemLibrary.Delay` 0.8)
  (`self.K2_DestroyActor`))

(fn `UserConstructionScript`)