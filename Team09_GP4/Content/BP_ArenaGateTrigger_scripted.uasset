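; Arena gate trigger that animates two gates when its box is overlapped and moves one again once all enemies are killed.
; The first overlap by any actor fires the OnPlayerOverlapped dispatcher, bound to OpenGates at BeginPlay, then unbinds it.
; Separate timelines drive each gate's relative Z, feeding world X/Y in as relative values.
; OnAllEnemiesKilled runs ClosedGate on Gate0 only; the player cast is unconnected and Opengate2 is empty.
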(event `self.ReceiveBeginPlay`
  (add `self.OnPlayerOverlapped` (delegate `Open gates`)))

(event `Open gates`
  (bind _gate (`self.Gate`))
  (bind _gate_0 (`self.Gate_0`))
  (bind (_returnvalue_x _returnvalue_y) (`KismetMathLibrary.BreakVector` (`self.K2_GetActorLocation` _gate_0)))
  (bind (_returnvalue_x_2 _returnvalue_y_2) (`KismetMathLibrary.BreakVector` (`self.K2_GetActorLocation` _gate)))
  (`|ExecutionSequence`
    (:`then_0`
      (bind (_direction _location) (`Timeline|Timeline`)
        (:`Update`
          (`self.K2_SetActorRelativeLocation` _gate (`KismetMathLibrary.MakeVector` _returnvalue_x_2 _returnvalue_y_2 _location) false false))))
    (:`then_1`
      (bind (_direction_2 _location_2) (`Timeline|Timeline_0`)
        (:`Update`
          (`self.K2_SetActorRelativeLocation` _gate_0 (`KismetMathLibrary.MakeVector` _returnvalue_x _returnvalue_y _location_2) false false))))))

(event `self.Box.OnComponentBeginOverlap`
  (params (OverlappedComponent :type "PrimitiveComponent Object Reference") (OtherActor :type "Actor Object Reference") (OtherComp :type "PrimitiveComponent Object Reference") (OtherBodyIndex :type Integer) (bFromSweep :type Boolean) (SweepResult :type "HitResult Structure (by ref)"))
  (`self.OnPlayerOverlapped`)
  (clear `self.OnPlayerOverlapped`))

(event `self.OnAllEnemiesKilled`
  (`self.Closed Gate`))

(event `Closed Gate`
  (bind _gate_0 (`self.Gate_0`))
  (bind (_returnvalue_x _returnvalue_y) (`KismetMathLibrary.BreakVector` (`self.K2_GetActorLocation` _gate_0)))
  (bind (_direction _location) (`Timeline|Timeline_1`)
    (:`Update`
      (`self.K2_SetActorRelativeLocation` _gate_0 (`KismetMathLibrary.MakeVector` _returnvalue_x _returnvalue_y _location) false false))))

(event `Open gate 2`)

(fn `UserConstructionScript`)